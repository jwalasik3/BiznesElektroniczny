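; BP_Architect is the player's bridge-building tool, aiming line traces from a pointer child actor, debug-drawn each tick.
; Interact starts a ballista, stores the first connectable hit point or links it to a second, and sends other hit actors an interact message.
; Connect spawns the selected segment type at the first point, rotated toward the second and X-scaled to span the gap.
; Right mouse destroys the targeted segment.
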(event EventBeginPlay)

(event Collision|EventActorBeginOverlap
  (params (OtherActor :type Actor%20Object%20Reference)))

(event EventTick
  (params (DeltaSeconds :type Float%20%28single-precision%29))
  (CallFunction|DoLineTrace))

(event Input|ActionEvents|InputActionInteract
  (params (Key :type Key%20Structure :default "None"))
  (:Pressed
    (bind (_hitactor _location) (CallFunction|DoLineTrace))
    (Development|PrintString (Utilities|GetDisplayName _hitactor))
    (bind _asbp_balista (Utilities|Casting|CastToBP_Balista _hitactor)
      (:then
        (Variables|/Game/Bridge/Balista/BP_Balista.BP_Balista_C|SetStarted _asbp_balista true))
      (:CastFailed
        (bind _asbp_connectable (Utilities|Casting|CastToBP_Connectable _hitactor)
          (:then
            (Utilities|IsValid (Variables|Default|GetFirstEnd)
              (:Is%20Valid
                (CallFunction|Connect (Variables|Default|GetFirstEnd) _asbp_connectable (Variables|Default|GetFirstEndLocation) _location))
              (:Is%20Not%20Valid
                (Variables|Default|SetFirstEnd _asbp_connectable)
                (Variables|Default|SetFirstEndLocation _location))))
          (:CastFailed
            (Class|InteractInterface|Interact(Message) _hitactor)))))))

(event Input|MouseEvents|RightMouseButton
  (params (Key :type Key%20Structure :default "None"))
  (:Pressed
    (bind _hitactor (CallFunction|DoLineTrace))
    (bind _asbp_segment (Utilities|Casting|CastToBP_Segment _hitactor))
    (Actor|DestroyActor _asbp_segment)))

(fn ConstructionScript
  (|CallParentFunction))

(fn DoLineTrace
  (bind _pointer_childactor (Variables|Default|GetPointer%20ChildActor))
  (bind _returnvalue (Transformation|GetWorldLocation _pointer_childactor))
  (bind _outactors (Actor|GetAllActorsOfClass "/Game/PointerBP.PointerBP_C"))
  (bind _outhit (Collision|LineTraceByChannel _returnvalue (+ _returnvalue (* (Math|Vector|GetForwardVector _pointer_childactor) 1e+03)) "TraceTypeQuery1" false _outactors "ForOneFrame"))
  (return (.HitActor (Collision|BreakHitResult _outhit)) (.Location (Collision|BreakHitResult _outhit))))

(fn Connect
  (params (NewParam :type BP%20Connectable%20Object%20Reference) (NewParam1 :type BP%20Connectable%20Object%20Reference) (NewParam2 :type Vector) (NewParam3 :type Vector))
  (bind _returnvalue (- NewParam3 NewParam2))
  (Game|SpawnActorfromClass (Variables|Default|GetSelectedSegmentType) (Math|Transform|MakeTransform NewParam2 (Math|Conversions|RotationFromXVector _returnvalue) (Math|Vector|MakeVector (/ (Math|Vector|VectorLength _returnvalue) 1e+02) 1.0 1.0)) "Undefined" "MultiplyWithRoot" 0 0)
  (Variables|Default|SetFirstEnd 0)
  (Development|PrintString "connected"))