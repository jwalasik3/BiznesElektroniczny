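; BP_Flystick0 represents a DTrack flystick in the CAVE, reading its button input and reacting to hand collision overlaps.
; On each LiveLink update it evaluates the flystick input role and caches button states to detect changes; the per-button press branches are empty stubs.
; Hand collision begin and end overlaps with components whose first tag is "collider" set the Sphere's material, with no material specified in either call.
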(event OnComponentBeginOverlap(Hand_colition)
  (params (OverlappedComponent :type Primitive%20Component%20Object%20Reference) (OtherActor :type Actor%20Object%20Reference) (OtherComp :type Primitive%20Component%20Object%20Reference) (OtherBodyIndex :type Integer) (bFromSweep :type Boolean) (SweepResult :type Hit%20Result%20Structure%20%28by%20ref%29))
  (if (== (Utilities|Array|Get(acopy) (Variables|/Script/Engine.ActorComponent|GetComponentTags OtherComp)) "collider")
    (Rendering|Material|SetMaterial (Variables|Default|GetSphere) 0 0)))

(event OnLiveLinkUpdated(LiveLink_Input)
  (params (DeltaTime :type Float%20%28single-precision%29))
  (bind _buttonstate_1 (Variables|Default|GetButtonState_1))
  (bind _dataresult (|EvaluateLiveLinkFramewithSpecificRole "(Name=\"DTrack-FlystickInput-00\")" "/Script/DTrackPlugin.DTrackFlystickInputRole")
    (:then
      (for (_array_element _array_index) (.m_button_state (.m_frame_data _dataresult))
        (if (!= _array_element (Utilities|Array|Get(acopy) _buttonstate_1 _array_index))
          (Utilities|Array|SetArrayElem _buttonstate_1 _array_index _array_element)
          (switch int _array_index
            (:0
              (if _array_element
                _))
            (:1
              (if _array_element
                _))
            (:2
              (if _array_element
                _))
            (:3
              (if _array_element
                _))
            (:4
              (if _array_element
                _))
            (:5
              (if _array_element
                _))))))))

(event OnComponentEndOverlap(Hand_colition)
  (params (OverlappedComponent :type Primitive%20Component%20Object%20Reference) (OtherActor :type Actor%20Object%20Reference) (OtherComp :type Primitive%20Component%20Object%20Reference) (OtherBodyIndex :type Integer))
  (if (== (Utilities|Array|Get(acopy) (Variables|/Script/Engine.ActorComponent|GetComponentTags OtherComp)) "collider")
    (Rendering|Material|SetMaterial (Variables|Default|GetSphere) 0 0)))

(fn ConstructionScript)